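; Enemy actor Blueprint that awards score to the player when it is shot, then destroys itself.
; BeginPlay caches the player ship pawn and the game instance.
; OnObjectShot adds ScoreValue to the pawn's current score, updates the game instance's high score if exceeded, and also adds the value to the instance's running player score.
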(event EventBeginPlay
  ;[1 1 1] Start
  (bind _asplayer_ship_pawn (Utilities|Casting|CastToPlayerShipPawn (Game|Player|GetPlayerPawn 0)))
  (Variables|Default|SetPlayerPawn _asplayer_ship_pawn)
  (bind _asnew_game_instance (Utilities|Casting|CastToNewGameInstance (Game|GetGameInstance)))
  (Variables|Default|SetInstance _asnew_game_instance))

(event Collision|EventActorBeginOverlap
  (params (OtherActor :type Actor%20Object%20Reference)))

(event EventTick
  (params (DeltaSeconds :type Float%20%28single-precision%29)))

(event EventOnObjectShot
  (bind _playerpawn (Variables|Default|GetPlayerPawn))
  (bind _scorevalue (Variables|Default|GetScoreValue))
  (bind _instance (Variables|Default|GetInstance))
  ;[1 1 1] When Enemy is Shot
  (bind _output_get (Variables|/Game/Blueprints/PlayerShipPawn.PlayerShipPawn_C|SetCurrentScore _playerpawn (+ (Variables|/Game/Blueprints/PlayerShipPawn.PlayerShipPawn_C|GetCurrentScore _playerpawn) _scorevalue)))
  (CallFunction|CheckforHighScore _output_get)
  (Variables|/Game/Blueprints/NewGameInstance.NewGameInstance_C|SetCurrentPlayerScore _instance (+ (Variables|/Game/Blueprints/NewGameInstance.NewGameInstance_C|GetCurrentPlayerScore _instance) _scorevalue))
  (Actor|DestroyActor))

(fn ConstructionScript)

(fn CheckforHighScore
  (params (IncomingScore :type Integer))
  (bind _instance (Variables|Default|GetInstance))
  (if (> IncomingScore (Variables|/Game/Blueprints/NewGameInstance.NewGameInstance_C|GetHighScore _instance))
    (Variables|/Game/Blueprints/NewGameInstance.NewGameInstance_C|SetHighScore _instance IncomingScore)))