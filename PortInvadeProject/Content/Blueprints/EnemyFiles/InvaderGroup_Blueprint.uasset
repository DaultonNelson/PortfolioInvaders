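; Space Invaders-style enemy formation that spawns five rows of eleven invaders, typed from a data table, with speed and fire rate scaled by level.
; Tick marches the group sideways, dropping and reversing at boundaries, and fires from random survivors after a delay.
; Per-column arrays let recursive edge checks widen boundaries as outer columns empty.
; Removing invaders speeds up movement, sharply for the last one; clearing all stops play and reloads GameplayScene.
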(event EventBeginPlay
  ;[1 1 1] Spawning Everything In
  (bind _asnew_game_instance (Utilities|Casting|CastToNewGameInstance (Game|GetGameInstance)))
  (Variables|Default|SetInstance _asnew_game_instance)
  (bind _asplayer_ship_pawn (Utilities|Casting|CastToPlayerShipPawn (Game|Player|GetPlayerPawn 0)))
  (Variables|Default|SetPlayerPawn _asplayer_ship_pawn)
  (for _index (range 0 4)
    (Variables|Default|SetSpawnZValue (Math|Conversions|ToFloat(Integer) (* _index 60)))
    (switch int _index
      (:Default
        (Development|PrintString "Index not valid" true true "(R=1.000000,G=0.000000,B=0.015027,A=1.000000)" 1e+01))
      (:0
        (Variables|Default|SetEnemyType "Brain" :!label _label)
        (for _index_2 (range 1 11) :!label _label_2
          (CallFunction|CycleThroughXValues _index_2)
          (bind _returnvalue (Game|SpawnActorfromClass "/Game/Blueprints/EnemyFiles/EnemyPrefab.EnemyPrefab_C" (Math|Conversions|ToTransform(Vector) (Math|Vector|MakeVector (Variables|Default|GetSpawnXValue) 0.0 (Variables|Default|GetSpawnZValue))) "Undefined" self 0 0))
          (Variables|Default|SetSpawnedEnemy _returnvalue)
          (Utilities|Array|Add (Variables|Default|GetChildInvaders_General) _returnvalue)
          (CallFunction|AddtoColumnBasedonIndex _index_2)
          (Transformation|AttachActorToActor (Variables|Default|GetSpawnedEnemy) self "None" "KeepRelative" "KeepRelative" "KeepRelative" true)
          (bind _returnvalue_2 (Utilities|GetDataTableRow (Variables|Default|GetEnemyTable) (Utilities|String|StringToName (Variables|Default|GetEnemyType)))
            (:then
              (Variables|/Game/Blueprints/EnemyFiles/Base_Enemy.Base_Enemy_C|SetScoreValue (Variables|Default|GetSpawnedEnemy) (.EnemyScore (Utilities|Struct|BreakEnemyStruct _returnvalue_2)))
              (Class|SkinnedMeshComponent|SetSkeletalMesh (Variables|/Game/Blueprints/EnemyFiles/EnemyPrefab.EnemyPrefab_C|GetEnemySkeleton (Variables|Default|GetSpawnedEnemy)) (.EnemyMesh (Utilities|Struct|BreakEnemyStruct _returnvalue_2)) true)
              (Components|SkeletalMesh|SetAnimInstanceClass (Variables|/Game/Blueprints/EnemyFiles/EnemyPrefab.EnemyPrefab_C|GetEnemySkeleton (Variables|Default|GetSpawnedEnemy)) (.EnemyAnimation (Utilities|Struct|BreakEnemyStruct _returnvalue_2)))
              (Variables|/Game/Blueprints/EnemyFiles/EnemyPrefab.EnemyPrefab_C|SetInvaderParent (Variables|Default|GetSpawnedEnemy) self)))))
      (:1
        (goto _label))
      (:2
        (Variables|Default|SetEnemyType "Bug" :!label _label_3)
        (goto _label_2))
      (:3
        (goto _label_3))
      (:4
        (Variables|Default|SetEnemyType "Squid")
        (goto _label_2))))
  (CallFunction|ColumnStatusCheck)
  (CallFunction|DifficultySetup))

(event Collision|EventActorBeginOverlap
  (params (OtherActor :type Actor%20Object%20Reference)))

(event EventTick
  (params (DeltaSeconds :type Float%20%28single-precision%29))
  (bind _childinvaders_general (Variables|Default|GetChildInvaders_General))
  (if (Math|Boolean|Equal(Boolean) (Variables|/Game/Blueprints/GameMode_SHUMP_Files/NewGameInstance.NewGameInstance_C|GetStopEverything (Variables|Default|GetInstance)) false)
    (CallFunction|GroupMovement DeltaSeconds)
    ;[1 1 1] Shooting
    (Utilities|FlowControl|Delay (Variables|Default|GetTimeBetweenShots))
    (Default|ShootLaser (Utilities|Array|Get(acopy) _childinvaders_general (Math|Random|RandomIntegerinRange 0 (- (Utilities|Array|Length _childinvaders_general) 1))))))

(fn ConstructionScript)

(fn CheckEven/Odd
  (params (Value :type Integer))
  (if (== Value 0)
    (return false)
    (elif (!= (Math|Integer|%(Integer) Value 2) 0)
      (return false)
      (else
        (return true)))))

(fn CycleThroughXValues
  (params (Index :type Integer))
  (if (== Index 1)
    (Variables|Default|SetSpawnXValue 0.0))
  (bind _iseven (CallFunction|CheckEven/Odd Index))
  (if _iseven
    (if (== (Math|Float|Sign(Float) (Variables|Default|GetSpawnXValue)) 1.0)
      (Variables|Default|SetSpawnXValue (+ (Variables|Default|GetSpawnXValue) 6e+01))
      (else
        (Variables|Default|SetSpawnXValue (- (Variables|Default|GetSpawnXValue) 6e+01))))
    (else
      (bind _result (Math|Float|NegateFloat (Variables|Default|GetSpawnXValue))
        (:%20%20
          (Variables|Default|SetSpawnXValue _result))))))

(fn AddtoColumnBasedonIndex
  (params (Index :type Integer))
  (switch int Index
    (:Default
      (Development|PrintString "Index not valid" true true "(R=1.000000,G=0.000000,B=0.015027,A=1.000000)" 1e+01))
    (:1
      ;[1 1 1] Col 6
      (Utilities|Array|Add (Variables|Default|GetChildInvaders_Col_6) (Variables|Default|GetSpawnedEnemy)))
    (:2
      ;[1 1 1] Col 5
      (Utilities|Array|Add (Variables|Default|GetChildInvaders_Col_5) (Variables|Default|GetSpawnedEnemy)))
    (:3
      ;[1 1 1] Col 7
      (Utilities|Array|Add (Variables|Default|GetChildInvaders_Col_7) (Variables|Default|GetSpawnedEnemy)))
    (:4
      ;[1 1 1] Col 8
      (Utilities|Array|Add (Variables|Default|GetChildInvaders_Col_8) (Variables|Default|GetSpawnedEnemy)))
    (:5
      ;[1 1 1] Col 4
      (Utilities|Array|Add (Variables|Default|GetChildInvaders_Col_4) (Variables|Default|GetSpawnedEnemy)))
    (:6
      ;[1 1 1] Col 3
      (Utilities|Array|Add (Variables|Default|GetChildInvaders_Col_3) (Variables|Default|GetSpawnedEnemy)))
    (:7
      ;[1 1 1] Col 9
      (Utilities|Array|Add (Variables|Default|GetChildInvaders_Col_9) (Variables|Default|GetSpawnedEnemy)))
    (:8
      ;[1 1 1] Col 10
      (Utilities|Array|Add (Variables|Default|GetChildInvaders_Col_10) (Variables|Default|GetSpawnedEnemy)))
    (:9
      ;[1 1 1] Col 2
      (Utilities|Array|Add (Variables|Default|GetChildInvaders_Col_2) (Variables|Default|GetSpawnedEnemy)))
    (:10
      ;[1 1 1] Col 1
      (Utilities|Array|Add (Variables|Default|GetChildInvaders_Col_1) (Variables|Default|GetSpawnedEnemy)))
    (:11
      ;[1 1 1] Col 11
      (Utilities|Array|Add (Variables|Default|GetChildInvaders_Col_11) (Variables|Default|GetSpawnedEnemy)))))

(fn GroupMovement
  (params (DeltaTime :type Float%20%28single-precision%29))
  (bind _self self)
  (bind _movementspeed (Variables|Default|GetMovementSpeed))
  (bind _staticmeshcomponent (Variables|Debug|GetStaticMeshComponent _self))
  (bind _relativelocation (Variables|/Script/Engine.SceneComponent|GetRelativeLocation _staticmeshcomponent))
  (bind (_x _y _z) (Math|Vector|BreakVector _relativelocation))
  ;[1 1 1] Movement
  (if (<= (Math|Float|Absolute(Float) _x) 5.0)
    (Variables|Default|SetCanDown true))
  (if (or (<= _x (Variables|Default|GetLeftBoundryValue)) (>= _x (Variables|Default|GetRightBoundryValue))) ; Boundary Check
    (if (Variables|Default|GetCanDown) ; Can Down Check
      (Math|Float|NegateFloat _movementspeed
        (:%20%20
          (Transformation|SetRelativeLocation _staticmeshcomponent (Math|Vector|MakeVector _x _y (- _z (Variables|Default|GetLoweringValue))) false false)
          (Variables|Default|SetCanDown false)
          (Transformation|SetRelativeLocation _staticmeshcomponent (+ _relativelocation (* (* (Math|Vector|GetForwardVector _staticmeshcomponent) _movementspeed) DeltaTime)) false false :!label _label))))
    (else
      (goto _label))))

(fn ColumnStatusCheck
  (CallFunction|CheckColumnfromLeft)
  (CallFunction|CheckColumnfromRight))

(fn CheckColumnfromLeft
  (Development|PrintString (Utilities|String|ToString(Integer) (Variables|Default|GetCurrentActiveLeftColumn)) true true "(R=1.000000,G=0.905880,B=0.913848,A=1.000000)")
  ;[1 1 1] From Left
  (switch int (Variables|Default|GetCurrentActiveLeftColumn)
    (:Default
      (Development|PrintString "Column is either invalid or equal to 12" true true "(R=1.000000,G=0.632717,B=0.000000,A=1.000000)"))
    (:1
      (if (== (Utilities|Array|Length (Variables|Default|GetChildInvaders_Col_1)) 0)
        (bind _result (Math|Integer|IncrementInt (Variables|Default|GetCurrentActiveLeftColumn))
          (:%20%20
            (Variables|Default|SetCurrentActiveLeftColumn _result)
            (Variables|Default|SetLeftBoundryValue -160.669998)
            (CallFunction|CheckColumnfromLeft)))
        (else
          (Development|PrintString "Column 1 has values in it")
          (Variables|Default|SetLeftBoundryValue -100.099998))))
    (:2
      (if (== (Utilities|Array|Length (Variables|Default|GetChildInvaders_Col_2)) 0)
        (bind _result_2 (Math|Integer|IncrementInt (Variables|Default|GetCurrentActiveLeftColumn))
          (:%20%20
            (Variables|Default|SetCurrentActiveLeftColumn _result_2)
            (Variables|Default|SetLeftBoundryValue -219.929993)
            (CallFunction|CheckColumnfromLeft)))
        (else
          (Development|PrintString "Column 2 has values in it")
          (Variables|Default|SetLeftBoundryValue -160.669998))))
    (:3
      (if (== (Utilities|Array|Length (Variables|Default|GetChildInvaders_Col_3)) 0)
        (bind _result_3 (Math|Integer|IncrementInt (Variables|Default|GetCurrentActiveLeftColumn))
          (:%20%20
            (Variables|Default|SetCurrentActiveLeftColumn _result_3)
            (Variables|Default|SetLeftBoundryValue -280.26001)
            (CallFunction|CheckColumnfromLeft)))
        (else
          (Development|PrintString "Column 3 has values in it")
          (Variables|Default|SetLeftBoundryValue -219.929993))))
    (:4
      (if (== (Utilities|Array|Length (Variables|Default|GetChildInvaders_Col_4)) 0)
        (bind _result_4 (Math|Integer|IncrementInt (Variables|Default|GetCurrentActiveLeftColumn))
          (:%20%20
            (Variables|Default|SetCurrentActiveLeftColumn _result_4)
            (Variables|Default|SetLeftBoundryValue -340.459991)
            (CallFunction|CheckColumnfromLeft)))
        (else
          (Development|PrintString "Column 4 has values in it")
          (Variables|Default|SetLeftBoundryValue -280.26001))))
    (:5
      (if (== (Utilities|Array|Length (Variables|Default|GetChildInvaders_Col_5)) 0)
        (bind _result_5 (Math|Integer|IncrementInt (Variables|Default|GetCurrentActiveLeftColumn))
          (:%20%20
            (Variables|Default|SetCurrentActiveLeftColumn _result_5)
            (Variables|Default|SetLeftBoundryValue -400.359985)
            (CallFunction|CheckColumnfromLeft)))
        (else
          (Development|PrintString "Column 5 has values in it")
          (Variables|Default|SetLeftBoundryValue -340.459991))))
    (:6
      (if (== (Utilities|Array|Length (Variables|Default|GetChildInvaders_Col_6)) 0)
        (bind _result_6 (Math|Integer|IncrementInt (Variables|Default|GetCurrentActiveLeftColumn))
          (:%20%20
            (Variables|Default|SetCurrentActiveLeftColumn _result_6)
            (Variables|Default|SetLeftBoundryValue -460.299988)
            (CallFunction|CheckColumnfromLeft)))
        (else
          (Development|PrintString "Column 6 has values in it")
          (Variables|Default|SetLeftBoundryValue -400.359985))))
    (:7
      (if (== (Utilities|Array|Length (Variables|Default|GetChildInvaders_Col_7)) 0)
        (bind _result_7 (Math|Integer|IncrementInt (Variables|Default|GetCurrentActiveLeftColumn))
          (:%20%20
            (Variables|Default|SetCurrentActiveLeftColumn _result_7)
            (Variables|Default|SetLeftBoundryValue -520.309998)
            (CallFunction|CheckColumnfromLeft)))
        (else
          (Development|PrintString "Column 7 has values in it")
          (Variables|Default|SetLeftBoundryValue -460.299988))))
    (:8
      (if (== (Utilities|Array|Length (Variables|Default|GetChildInvaders_Col_8)) 0)
        (bind _result_8 (Math|Integer|IncrementInt (Variables|Default|GetCurrentActiveLeftColumn))
          (:%20%20
            (Variables|Default|SetCurrentActiveLeftColumn _result_8)
            (Variables|Default|SetLeftBoundryValue -580.320007)
            (CallFunction|CheckColumnfromLeft)))
        (else
          (Development|PrintString "Column 8 has values in it")
          (Variables|Default|SetLeftBoundryValue -520.309998))))
    (:9
      (if (== (Utilities|Array|Length (Variables|Default|GetChildInvaders_Col_9)) 0)
        (bind _result_9 (Math|Integer|IncrementInt (Variables|Default|GetCurrentActiveLeftColumn))
          (:%20%20
            (Variables|Default|SetCurrentActiveLeftColumn _result_9)
            (Variables|Default|SetLeftBoundryValue -640.330017)
            (CallFunction|CheckColumnfromLeft)))
        (else
          (Development|PrintString "Column 9 has values in it")
          (Variables|Default|SetLeftBoundryValue -580.320007))))
    (:10
      (if (== (Utilities|Array|Length (Variables|Default|GetChildInvaders_Col_10)) 0)
        (bind _result_10 (Math|Integer|IncrementInt (Variables|Default|GetCurrentActiveLeftColumn))
          (:%20%20
            (Variables|Default|SetCurrentActiveLeftColumn _result_10)
            (Variables|Default|SetLeftBoundryValue -700.340027)
            (CallFunction|CheckColumnfromLeft)))
        (else
          (Development|PrintString "Column 10 has values in it")
          (Variables|Default|SetLeftBoundryValue -640.330017))))
    (:11
      (if (== (Utilities|Array|Length (Variables|Default|GetChildInvaders_Col_11)) 0)
        (bind _result_11 (Math|Integer|IncrementInt (Variables|Default|GetCurrentActiveLeftColumn))
          (:%20%20
            (Variables|Default|SetCurrentActiveLeftColumn _result_11)
            (Variables|Default|SetLeftBoundryValue -760.599976)
            (CallFunction|CheckColumnfromLeft)))
        (else
          (Development|PrintString "Column 11 has values in it")
          (Variables|Default|SetLeftBoundryValue -700.340027))))))

(fn CheckColumnfromRight
  (Development|PrintString (Utilities|String|ToString(Integer) (Variables|Default|GetCurrentActiveRightColumn)) true true "(R=1.000000,G=0.000000,B=0.867200,A=1.000000)")
  ;[1 1 1] From Right
  (switch int (Variables|Default|GetCurrentActiveRightColumn)
    (:Default
      (Development|PrintString "Column is either invalid or equal to 0" true true "(R=1.000000,G=0.632717,B=0.000000,A=1.000000)"))
    (:1
      (if (== (Utilities|Array|Length (Variables|Default|GetChildInvaders_Col_1)) 0)
        (bind _result (Math|Integer|DecrementInt (Variables|Default|GetCurrentActiveRightColumn))
          (:%20%20
            (Variables|Default|SetCurrentActiveRightColumn _result)
            (Variables|Default|SetRightBoundryValue 756.200012)
            (CallFunction|CheckColumnfromRight)))
        (else
          (Development|PrintString "Column 1 has values in it")
          (Variables|Default|SetRightBoundryValue 695.969971))))
    (:2
      (if (== (Utilities|Array|Length (Variables|Default|GetChildInvaders_Col_2)) 0)
        (bind _result_2 (Math|Integer|DecrementInt (Variables|Default|GetCurrentActiveRightColumn))
          (:%20%20
            (Variables|Default|SetCurrentActiveRightColumn _result_2)
            (Variables|Default|SetRightBoundryValue 695.969971)
            (CallFunction|CheckColumnfromRight)))
        (else
          (Development|PrintString "Column 2 has values in it")
          (Variables|Default|SetRightBoundryValue 635.960022))))
    (:3
      (if (== (Utilities|Array|Length (Variables|Default|GetChildInvaders_Col_3)) 0)
        (bind _result_3 (Math|Integer|DecrementInt (Variables|Default|GetCurrentActiveRightColumn))
          (:%20%20
            (Variables|Default|SetCurrentActiveRightColumn _result_3)
            (Variables|Default|SetRightBoundryValue 635.960022)
            (CallFunction|CheckColumnfromRight)))
        (else
          (Development|PrintString "Column 3 has values in it")
          (Variables|Default|SetRightBoundryValue 575.619995))))
    (:4
      (if (== (Utilities|Array|Length (Variables|Default|GetChildInvaders_Col_4)) 0)
        (bind _result_4 (Math|Integer|DecrementInt (Variables|Default|GetCurrentActiveRightColumn))
          (:%20%20
            (Variables|Default|SetCurrentActiveRightColumn _result_4)
            (Variables|Default|SetRightBoundryValue 575.619995)
            (CallFunction|CheckColumnfromRight)))
        (else
          (Development|PrintString "Column 4 has values in it")
          (Variables|Default|SetRightBoundryValue 515.609985))))
    (:5
      (if (== (Utilities|Array|Length (Variables|Default|GetChildInvaders_Col_5)) 0)
        (bind _result_5 (Math|Integer|DecrementInt (Variables|Default|GetCurrentActiveRightColumn))
          (:%20%20
            (Variables|Default|SetCurrentActiveRightColumn _result_5)
            (Variables|Default|SetRightBoundryValue 515.609985)
            (CallFunction|CheckColumnfromRight)))
        (else
          (Development|PrintString "Column 5 has values in it")
          (Variables|Default|SetRightBoundryValue 455.890015))))
    (:6
      (if (== (Utilities|Array|Length (Variables|Default|GetChildInvaders_Col_6)) 0)
        (bind _result_6 (Math|Integer|DecrementInt (Variables|Default|GetCurrentActiveRightColumn))
          (:%20%20
            (Variables|Default|SetCurrentActiveRightColumn _result_6)
            (Variables|Default|SetRightBoundryValue 455.890015)
            (CallFunction|CheckColumnfromRight)))
        (else
          (Development|PrintString "Column 6 has values in it")
          (Variables|Default|SetRightBoundryValue 396.480011))))
    (:7
      (if (== (Utilities|Array|Length (Variables|Default|GetChildInvaders_Col_7)) 0)
        (bind _result_7 (Math|Integer|DecrementInt (Variables|Default|GetCurrentActiveRightColumn))
          (:%20%20
            (Variables|Default|SetCurrentActiveRightColumn _result_7)
            (Variables|Default|SetRightBoundryValue 396.480011)
            (CallFunction|CheckColumnfromRight)))
        (else
          (Development|PrintString "Column 7 has values in it")
          (Variables|Default|SetRightBoundryValue 336.01001))))
    (:8
      (if (== (Utilities|Array|Length (Variables|Default|GetChildInvaders_Col_8)) 0)
        (bind _result_8 (Math|Integer|DecrementInt (Variables|Default|GetCurrentActiveRightColumn))
          (:%20%20
            (Variables|Default|SetCurrentActiveRightColumn _result_8)
            (Variables|Default|SetRightBoundryValue 336.01001)
            (CallFunction|CheckColumnfromRight)))
        (else
          (Development|PrintString "Column 8 has values in it")
          (Variables|Default|SetRightBoundryValue 276.029999))))
    (:9
      (if (== (Utilities|Array|Length (Variables|Default|GetChildInvaders_Col_9)) 0)
        (bind _result_9 (Math|Integer|DecrementInt (Variables|Default|GetCurrentActiveRightColumn))
          (:%20%20
            (Variables|Default|SetCurrentActiveRightColumn _result_9)
            (Variables|Default|SetRightBoundryValue 276.029999)
            (CallFunction|CheckColumnfromRight)))
        (else
          (Development|PrintString "Column 9 has values in it")
          (Variables|Default|SetRightBoundryValue 216.669998))))
    (:10
      (if (== (Utilities|Array|Length (Variables|Default|GetChildInvaders_Col_10)) 0)
        (bind _result_10 (Math|Integer|DecrementInt (Variables|Default|GetCurrentActiveRightColumn))
          (:%20%20
            (Variables|Default|SetCurrentActiveRightColumn _result_10)
            (Variables|Default|SetRightBoundryValue 216.669998)
            (CallFunction|CheckColumnfromRight)))
        (else
          (Development|PrintString "Column 10 has values in it")
          (Variables|Default|SetRightBoundryValue 156.270004))))
    (:11
      (if (== (Utilities|Array|Length (Variables|Default|GetChildInvaders_Col_11)) 0)
        (bind _result_11 (Math|Integer|DecrementInt (Variables|Default|GetCurrentActiveRightColumn))
          (:%20%20
            (Variables|Default|SetCurrentActiveRightColumn _result_11)
            (Variables|Default|SetRightBoundryValue 156.270004)
            (CallFunction|CheckColumnfromRight)))
        (else
          (Development|PrintString "Column 11 has values in it")
          (Variables|Default|SetRightBoundryValue 96.980003))))))

(fn RemovefromColumn
  (params (InvaderToRemove :type Enemy%20Prefab%20Object%20Reference))
  (bind _childinvaders_col_2 (Variables|Default|GetChildInvaders_Col_2))
  (bind _childinvaders_col_11 (Variables|Default|GetChildInvaders_Col_11))
  (bind _childinvaders_general (Variables|Default|GetChildInvaders_General))
  (bind _childinvaders_col_1 (Variables|Default|GetChildInvaders_Col_1))
  (bind _childinvaders_col_3 (Variables|Default|GetChildInvaders_Col_3))
  (bind _childinvaders_col_4 (Variables|Default|GetChildInvaders_Col_4))
  (bind _childinvaders_col_5 (Variables|Default|GetChildInvaders_Col_5))
  (bind _childinvaders_col_6 (Variables|Default|GetChildInvaders_Col_6))
  (bind _childinvaders_col_7 (Variables|Default|GetChildInvaders_Col_7))
  (bind _childinvaders_col_8 (Variables|Default|GetChildInvaders_Col_8))
  (bind _childinvaders_col_9 (Variables|Default|GetChildInvaders_Col_9))
  (bind _childinvaders_col_10 (Variables|Default|GetChildInvaders_Col_10))
  (bind _returnvalue (Utilities|Array|Length _childinvaders_general))
  ;[1 1 1] Dynamic Movement Incrementation
  (if (Utilities|Array|ContainsItem _childinvaders_general InvaderToRemove)
    (Utilities|Array|RemoveItem _childinvaders_general InvaderToRemove)
    (if (> _returnvalue 1)
      (Variables|Default|SetMovementSpeed (* (Variables|Default|GetMovementSpeed) 1.01))
      (for _index (range 1 11) :!label _label
        (switch int _index
          (:Default
            ;[1 1 1] Check and Remove
            (Development|PrintString "Index is Invalid" true true "(R=1.000000,G=0.000000,B=0.000000,A=1.000000)"))
          (:1
            (if (Utilities|Array|ContainsItem _childinvaders_col_1 InvaderToRemove)
              (Utilities|Array|RemoveItem _childinvaders_col_1 InvaderToRemove)))
          (:2
            (if (Utilities|Array|ContainsItem _childinvaders_col_2 InvaderToRemove)
              (Utilities|Array|RemoveItem _childinvaders_col_2 InvaderToRemove)))
          (:3
            (if (Utilities|Array|ContainsItem _childinvaders_col_3 InvaderToRemove)
              (Utilities|Array|RemoveItem _childinvaders_col_3 InvaderToRemove)))
          (:4
            (if (Utilities|Array|ContainsItem _childinvaders_col_4 InvaderToRemove)
              (Utilities|Array|RemoveItem _childinvaders_col_4 InvaderToRemove)))
          (:5
            (if (Utilities|Array|ContainsItem _childinvaders_col_5 InvaderToRemove)
              (Utilities|Array|RemoveItem _childinvaders_col_5 InvaderToRemove)))
          (:6
            (if (Utilities|Array|ContainsItem _childinvaders_col_6 InvaderToRemove)
              (Utilities|Array|RemoveItem _childinvaders_col_6 InvaderToRemove)))
          (:7
            (if (Utilities|Array|ContainsItem _childinvaders_col_7 InvaderToRemove)
              (Utilities|Array|RemoveItem _childinvaders_col_7 InvaderToRemove)))
          (:8
            (if (Utilities|Array|ContainsItem _childinvaders_col_8 InvaderToRemove)
              (Utilities|Array|RemoveItem _childinvaders_col_8 InvaderToRemove)))
          (:9
            (if (Utilities|Array|ContainsItem _childinvaders_col_9 InvaderToRemove)
              (Utilities|Array|RemoveItem _childinvaders_col_9 InvaderToRemove)))
          (:10
            (if (Utilities|Array|ContainsItem _childinvaders_col_10 InvaderToRemove)
              (Utilities|Array|RemoveItem _childinvaders_col_10 InvaderToRemove)))
          (:11
            (if (Utilities|Array|ContainsItem _childinvaders_col_11 InvaderToRemove)
              (Utilities|Array|RemoveItem _childinvaders_col_11 InvaderToRemove)))))
      (elif (> _returnvalue 0)
        (Variables|Default|SetMovementSpeed (* 12 (Variables|Default|GetMovementSpeed)))
        (Variables|Default|SetLoweringValue (* 3 (Variables|Default|GetLoweringValue)))
        (goto _label)
        (else
          (Variables|/Game/Blueprints/GameMode_SHUMP_Files/NewGameInstance.NewGameInstance_C|SetStopEverything (Variables|Default|GetInstance) true)
          (Utilities|Time|SetTimerbyFunctionName 0 "PlayerWonTheLevel" 3.0))))
    (else
      (Development|PrintString "Object not in general list" true true "(R=1.000000,G=0.000000,B=0.005996,A=1.000000)")
      (goto _label))))

(fn PlayerWontheLevel
  (Game|OpenLevel(byName) "GameplayScene"))

(fn DifficultySetup
  (bind _instance (Variables|Default|GetInstance))
  (bind _currentlevel (Variables|/Game/Blueprints/GameMode_SHUMP_Files/NewGameInstance.NewGameInstance_C|GetCurrentLevel _instance))
  (bind _returnvalue (- _currentlevel 1))
  (Variables|Default|SetTimeBetweenShots (- (Variables|Default|GetTimeBetweenShots) (* _returnvalue (Variables|Default|GetTimeShotIncrementValue))))
  (Variables|Default|SetMovementSpeed (+ (Variables|Default|GetMovementSpeed) (* _returnvalue (Variables|Default|GetMovementIncrementValue)))))