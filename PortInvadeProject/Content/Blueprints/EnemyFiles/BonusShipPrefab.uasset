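; BonusShipPrefab is a bonus enemy ship that travels in a straight line and awards score when shot.
; BeginPlay runs EnemySetup, and Tick moves the root component along world +X by MovementSpeed scaled by delta time, without sweeping.
; OnObjectShot calls ScoreHandling and then destroys the actor.
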(event EventBeginPlay
  ;[1 1 1] Setup
  (CallFunction|EnemySetup))

(event EventTick
  (params (DeltaSeconds :type Float%20%28single-precision%29))
  (bind _defaultsceneroot (Variables|Default|GetDefaultSceneRoot))
  ;[1 1 1] Movement
  (Transformation|SetWorldLocation _defaultsceneroot (+ (* (* "1.000000, 0, 0" (Variables|Default|GetMovementSpeed)) DeltaSeconds) (Transformation|GetWorldLocation _defaultsceneroot)) false false))

(event EventOnObjectShot
  ;[1 1 1] OnObjectShot
  (CallFunction|ScoreHandling)
  (Actor|DestroyActor))

(fn ConstructionScript)