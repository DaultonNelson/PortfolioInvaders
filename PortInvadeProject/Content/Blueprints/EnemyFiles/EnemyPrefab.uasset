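; Enemy invader prefab that can fire lasers and explodes when shot, reporting to an InvaderParent that tracks enemies by column.
; BeginPlay runs EnemySetup, and ShootLaser spawns an enemy laser at the skeletal mesh's transform.
; OnObjectShot handles score, runs DeathBehavior, plays a sound and destroys the actor after a delay.
; DeathBehavior, guarded by Killed, removes collision and column entry, triggers red-tinted particles through a dynamic material, and hides the mesh.
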(event EventBeginPlay
  ;[1 1 1] Start
  (CallFunction|EnemySetup))

(event Collision|EventActorBeginOverlap
  (params (OtherActor :type Actor%20Object%20Reference)))

(event EventTick
  (params (DeltaSeconds :type Float%20%28single-precision%29)))

(event EventOnObjectShot
  ;[1 1 1] When Enemy is Shot
  (CallFunction|ScoreHandling)
  (CallFunction|DeathBehavior)
  (Audio|PlaySound2D "/Game/Sounds/Enemy_Explosion_Cue.Enemy_Explosion_Cue" 1.0 1.0 0.0 0 0)
  (Utilities|FlowControl|Delay 1.0)
  (Actor|DestroyActor))

(fn ConstructionScript
  (Variables|Default|SetEnemySkeleton (Variables|Default|GetSkeletalMesh)))

(fn ShootLaser
  (bind _returnvalue (Game|SpawnActorfromClass "/Game/Blueprints/EnemyFiles/Child_Laser_Blueprint_Enemy.Child_Laser_Blueprint_Enemy_C" (Transformation|GetWorldTransform (Variables|Default|GetSkeletalMesh self)) "Undefined" 0 0))
  (Variables|Default|SetSpawnedLaser _returnvalue))

(fn DeathBehavior
  (bind _explosionsystem (Variables|Default|GetExplosionSystem))
  (bind _invaderparent (Variables|Default|GetInvaderParent))
  (if (not (Variables|Default|GetKilled))
    (Variables|Default|SetKilled true)
    (Components|DestroyComponent (Variables|Default|GetBoxCollision))
    (Default|RemovefromColumn _invaderparent self)
    (Default|ColumnStatusCheck _invaderparent)
    (bind _returnvalue (Rendering|Material|CreateDynamicMaterialInstance _explosionsystem 0 "/Game/Materials/FireworksDot_M.FireworksDot_M" "None" :!class /Script/Engine.PrimitiveComponent))
    (Rendering|Material|SetVectorParameterValue _returnvalue "Color" (Utilities|Struct|MakeLinearColor 1.0 0.0 0.0 1.0) :!class /Script/Engine.MaterialInstanceDynamic)
    (Rendering|Material|SetMaterial _explosionsystem 0 _returnvalue)
    (Rendering|Material|SetMaterial _explosionsystem 1 _returnvalue)
    (Components|Activation|Activate _explosionsystem false)
    (Rendering|ToggleVisibility (Variables|Default|GetSkeletalMesh) false)))