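; Base_Enemy is an enemy Blueprint providing shared setup and score handling.
; EnemySetup casts and caches the custom player controller, player ship pawn and game instance.
; ScoreHandling adds the enemy's ScoreValue to the game instance score and updates the high score through CheckForHighScore.
; Crossing the next-life threshold plays a sound, grants a life, rebuilds the lives widget and raises the threshold by a fixed step.
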(fn ConstructionScript)

(fn ScoreHandling
  (bind _instance (Variables|Default|GetInstance))
  (bind _output_get (Variables|/Game/Blueprints/GameMode_SHUMP_Files/NewGameInstance.NewGameInstance_C|SetCurrentPlayerScore _instance (+ (Variables|/Game/Blueprints/GameMode_SHUMP_Files/NewGameInstance.NewGameInstance_C|GetCurrentPlayerScore _instance) (Variables|Default|GetScoreValue))))
  (CallFunction|CheckforHighScore _output_get)
  (if (>= _output_get (Variables|/Game/Blueprints/GameMode_SHUMP_Files/NewGameInstance.NewGameInstance_C|GetNextLifeValue _instance))
    (Audio|PlaySound2D "/Game/Sounds/Gain_Life_Cue.Gain_Life_Cue" 1.0 1.0 0.0 0 0)
    (Math|Integer|IncrementInt (Variables|/Game/Blueprints/GameMode_SHUMP_Files/NewGameInstance.NewGameInstance_C|GetPlayerLives _instance)
      (:%20%20
        (Default|RebuildLives (Variables|/Game/Blueprints/GameMode_SHUMP_Files/CustomPlayerController.CustomPlayerController_C|GetGameplayWidget (Variables|Default|GetPlayController)))
        (Variables|/Game/Blueprints/GameMode_SHUMP_Files/NewGameInstance.NewGameInstance_C|SetNextLifeValue _instance (+ (Variables|/Game/Blueprints/GameMode_SHUMP_Files/NewGameInstance.NewGameInstance_C|GetNextLifeValue _instance) 1500))))))

(fn CheckforHighScore
  (params (IncomingScore :type Integer))
  (bind _instance (Variables|Default|GetInstance))
  (if (> IncomingScore (Variables|/Game/Blueprints/GameMode_SHUMP_Files/NewGameInstance.NewGameInstance_C|GetHighScore _instance))
    (Variables|/Game/Blueprints/GameMode_SHUMP_Files/NewGameInstance.NewGameInstance_C|SetNewHighScore _instance true)
    (Variables|/Game/Blueprints/GameMode_SHUMP_Files/NewGameInstance.NewGameInstance_C|SetHighScore _instance IncomingScore)
    (return)
    (else
      (return))))

(fn EnemySetup
  (bind _ascustom_player_controller (Utilities|Casting|CastToCustomPlayerController (Game|GetPlayerController 0)))
  (Variables|Default|SetPlayController _ascustom_player_controller)
  (bind _asplayer_ship_pawn (Utilities|Casting|CastToPlayerShipPawn (Game|Player|GetPlayerPawn 0)))
  (Variables|Default|SetPlayerPawn _asplayer_ship_pawn)
  (bind _asnew_game_instance (Utilities|Casting|CastToNewGameInstance (Game|GetGameInstance)))
  (Variables|Default|SetInstance _asnew_game_instance))