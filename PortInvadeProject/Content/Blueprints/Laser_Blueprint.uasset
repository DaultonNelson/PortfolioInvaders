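; Laser projectile actor that flies in a straight line and notifies shootable objects it hits.
; Tick moves it along its up vector by LaserSpeed, without sweep or delta-time scaling.
; Capsule overlap sends OnObjectShotMessage to actors implementing BPI_Shootable, then destroys the laser.
; BeginPlay caches the mesh's material instance and destroys the laser after LaserLife, only if that material cast succeeds.
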(event OnComponentBeginOverlap(Capsule)
  (params (OverlappedComponent :type Primitive%20Component%20Object%20Reference) (OtherActor :type Actor%20Object%20Reference) (OtherComp :type Primitive%20Component%20Object%20Reference) (OtherBodyIndex :type Integer) (bFromSweep :type Boolean) (SweepResult :type Hit%20Result%20Structure%20%28by%20ref%29))
  (if (Utilities|DoesObjectImplementInterface OtherActor "/Game/Blueprints/BPI_Shootable.BPI_Shootable_C")
    (bind _output_get (Variables|Default|SetOverlappedActor OtherActor))
    (Class|BPIShootable|OnObjectShot(Message) _output_get)
    (Actor|DestroyActor)))

(event EventBeginPlay
  ;[1 1 1] Getting Material and Destroying after Delay
  (bind _asmaterial_instance (Utilities|Casting|CastToMaterialInstance (Rendering|Material|GetMaterial (Variables|Debug|GetStaticMeshComponent) 0)))
  (Variables|Default|SetLaserMaterial _asmaterial_instance)
  (Utilities|FlowControl|Delay (Variables|Default|GetLaserLife))
  (Actor|DestroyActor))

(event Collision|EventActorBeginOverlap
  (params (OtherActor :type Actor%20Object%20Reference)))

(event EventTick
  (params (DeltaSeconds :type Float%20%28single-precision%29))
  ;[1 1 1] Laser Movement
  (Transformation|SetActorLocation (+ (* (Transformation|GetActorUpVector) (Variables|Default|GetLaserSpeed)) (Transformation|GetActorLocation)) false false))

(fn ConstructionScript)