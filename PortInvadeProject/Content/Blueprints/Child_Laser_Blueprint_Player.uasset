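; Player laser projectile, a child Blueprint that damages enemies, bonus ships and shield pieces.
; It expires after LaserLife seconds and moves each Tick through LaserMovement.
; Capsule overlaps pass through OnLaserCollision, then a cast chain checks OverlappedActor for the three target types.
; A match receives OnObjectShotMessage and the laser destroys itself, while failed casts print debug strings.
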(event OnComponentBeginOverlap(Capsule)
  (params (OverlappedComponent :type Primitive%20Component%20Object%20Reference) (OtherActor :type Actor%20Object%20Reference) (OtherComp :type Primitive%20Component%20Object%20Reference) (OtherBodyIndex :type Integer) (bFromSweep :type Boolean) (SweepResult :type Hit%20Result%20Structure%20%28by%20ref%29))
  (bind _overlappedactor (Variables|Default|GetOverlappedActor))
  ;[1 1 1] Collision
  (bind _hasinterface (CallFunction|OnLaserCollision OtherActor))
  (if _hasinterface
    (Utilities|Casting|CastToEnemyPrefab _overlappedactor
      (:then
        (Class|BPIShootable|OnObjectShot(Message) _overlappedactor)
        (Actor|DestroyActor))
      (:CastFailed
        (Development|PrintString "Not an enemy prefab")
        (Utilities|Casting|CastToBonusShipPrefab _overlappedactor
          (:then
            (Class|BPIShootable|OnObjectShot(Message) _overlappedactor)
            (Actor|DestroyActor))
          (:CastFailed
            (Development|PrintString "Not a bonus ship")
            (Utilities|Casting|CastToShieldBlueprint _overlappedactor
              (:then
                (Class|BPIShootable|OnObjectShot(Message) _overlappedactor)
                (Actor|DestroyActor))
              (:CastFailed
                (Development|PrintString "Not a shield piece")))))))))

(event EventBeginPlay
  (Actor|SetLifeSpan (Variables|Default|GetLaserLife)))

(event Collision|EventActorBeginOverlap
  (params (OtherActor :type Actor%20Object%20Reference)))

(event EventTick
  (params (DeltaSeconds :type Float%20%28single-precision%29))
  (CallFunction|LaserMovement DeltaSeconds))

(fn ConstructionScript
  (|CallParentFunction))