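; Player ship pawn that slides along a clamped horizontal track, fires lasers and can be shot down.
; The horizontal axis offsets the ship mesh along its forward vector, with relative X clamped.
; Releasing Fire spawns a laser at the muzzle and tints it with a custom color through a dynamic material instance.
; OnObjectShot sets a dead flag that blocks input and destroys the ship and muzzle components, leaving the pawn itself.
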(event EventBeginPlay)

(event Collision|EventActorBeginOverlap
  (params (OtherActor :type Actor%20Object%20Reference)))

(event EventTick
  (params (DeltaSeconds :type Float%20%28single-precision%29)))

(event EventOnObjectShot
  ;[1 1 1] Killing the Player Ship
  (Variables|Default|SetIsDead true)
  (Components|DestroyComponent (Variables|Default|GetMuzzle))
  (Components|DestroyComponent (Variables|Default|GetPlayerShip)))

(event Input|ActionEvents|InputActionFire
  (params (Key :type Key%20Structure))
  ;[1 1 1] Shooting Lasers
  (:Released
    (if (not (Variables|Default|GetIsDead))
      (Development|PrintString "Fire Shot")
      (bind _returnvalue (Game|SpawnActorfromClass "/Game/Blueprints/Laser_Blueprint.Laser_Blueprint_C" (Transformation|GetWorldTransform (Variables|Default|GetMuzzle)) "Undefined" 0 0))
      (Variables|Default|SetSpawnedLaser _returnvalue)
      (bind _returnvalue_2 (Rendering|Material|CreateDynamicMaterialInstance (Variables|/Game/Blueprints/Laser_Blueprint.Laser_Blueprint_C|GetLaserMaterial _returnvalue) (Variables|/Game/Blueprints/Laser_Blueprint.Laser_Blueprint_C|GetLaserMaterial _returnvalue) "None" :!class /Script/Engine.KismetMaterialLibrary))
      (Rendering|Material|SetMaterial (Variables|/Script/Engine.StaticMeshActor|GetStaticMeshComponent (Variables|Default|GetSpawnedLaser)) 0 _returnvalue_2)
      (Rendering|Material|SetVectorParameterValue _returnvalue_2 "LaserColor" (Variables|Default|GetCustomLaserColor) :!class /Script/Engine.MaterialInstanceDynamic))))

(event Input|AxisEvents|InputAxisHorizontalAxis
  (params (AxisValue :type Float%20%28single-precision%29))
  (bind _playership (Variables|Default|GetPlayerShip))
  (bind _movementspeed (Variables|Default|GetMovementSpeed))
  (bind _returnvalue (Math|Vector|GetForwardVector _playership))
  (bind _relativelocation (Variables|/Script/Engine.SceneComponent|GetRelativeLocation _playership))
  (bind _returnvalue_2 (* _returnvalue AxisValue))
  (bind _returnvalue_3 (* _returnvalue_2 _movementspeed))
  (bind _returnvalue_4 (+ _returnvalue_3 _relativelocation))
  (bind (_x _y _z) (Math|Vector|BreakVector _returnvalue_4))
  ;[1 1 1] Ship Movement
  (if (not (Variables|Default|GetIsDead))
    (Transformation|SetRelativeLocation _playership (Math|Vector|MakeVector (Math|Float|Clamp(Float) _x -2e+02 2e+02) _y _z) false false)))

(fn ConstructionScript)