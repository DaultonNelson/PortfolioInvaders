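; Player satellite that slides along X and triggers game over when shot.
; BeginPlay caches the game instance and HUD widget and creates a save object; Tick moves the mesh, flipping speed at either edge, re-armed near center.
; Being shot hides the mesh, destroys its collider, fires a green-tinted explosion, sets the shared StopEverything flag, shows game-over text and saves any new high score.
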(event EventBeginPlay
  ;[1 1 1] Start
  (bind _asnew_game_instance (Utilities|Casting|CastToNewGameInstance (Game|GetGameInstance)))
  (Variables|Default|SetInstance _asnew_game_instance)
  (bind _ascustom_player_controller (Utilities|Casting|CastToCustomPlayerController (Game|GetPlayerController 0))
    (:then
      (Variables|Default|SetUIWidget (Variables|/Game/Blueprints/GameMode_SHUMP_Files/CustomPlayerController.CustomPlayerController_C|GetGameplayWidget _ascustom_player_controller))
      (bind _returnvalue (SaveGame|CreateSaveGameObject "/Game/Blueprints/ShumpSaveGame.ShumpSaveGame_C"))
      (Variables|Default|SetSave _returnvalue))
    (:CastFailed
      (Development|PrintString "Controller not found" true true "(R=0.537965,G=1.000000,B=0.538221,A=1.000000)" 99.0))))

(event Collision|EventActorBeginOverlap
  (params (OtherActor :type Actor%20Object%20Reference)))

(event EventTick
  (params (DeltaSeconds :type Float%20%28single-precision%29))
  (CallFunction|SatelliteMovement DeltaSeconds))

(event EventOnObjectShot
  (bind _uiwidget (Variables|Default|GetUIWidget))
  (bind _explosion (Variables|Default|GetExplosion))
  (bind _instance (Variables|Default|GetInstance))
  (bind _save (Variables|Default|GetSave))
  ;[1 1 1] When Object is Shot
  (Rendering|ToggleVisibility (Variables|Debug|GetStaticMeshComponent) false)
  (Components|DestroyComponent (Variables|Default|GetSphereCollider))
  (bind _returnvalue (Rendering|Material|CreateDynamicMaterialInstance _explosion 0 "/Game/Materials/FireworksDot_M.FireworksDot_M" "None" :!class /Script/Engine.PrimitiveComponent))
  (Rendering|Material|SetVectorParameterValue _returnvalue "Color" (Utilities|Struct|MakeLinearColor 0.0 1.0 0.0 1.0) :!class /Script/Engine.MaterialInstanceDynamic)
  (Rendering|Material|SetMaterial _explosion 0 _returnvalue)
  (Rendering|Material|SetMaterial _explosion 1 _returnvalue)
  (Components|Activation|Activate _explosion false)
  (Variables|/Game/Blueprints/GameMode_SHUMP_Files/NewGameInstance.NewGameInstance_C|SetStopEverything _instance true)
  (Rendering|Components|TextRender|SetText (Variables|/Game/UI/GameplayUI.GameplayUI_C|GetTextBlock_GameOverLabel _uiwidget) "GAME OVER, [SPACE] TO EXIT")
  (if (Variables|/Game/Blueprints/GameMode_SHUMP_Files/NewGameInstance.NewGameInstance_C|GetNewHighScore _instance)
    (Rendering|Components|TextRender|SetText (Variables|/Game/UI/GameplayUI.GameplayUI_C|GetTextBlock_NewHighScore _uiwidget) "NEW HI-SCORE GOT")
    (Variables|/Game/Blueprints/ShumpSaveGame.ShumpSaveGame_C|SetSavedHighScore _save (Variables|/Game/Blueprints/GameMode_SHUMP_Files/NewGameInstance.NewGameInstance_C|GetHighScore _instance))
    (SaveGame|SaveGametoSlot _save "A")))

(fn ConstructionScript)

(fn SatelliteMovement
  (params (Delta%20Time :type Float%20%28single-precision%29))
  (bind _movementspeed (Variables|Default|GetMovementSpeed))
  (bind _staticmeshcomponent (Variables|Debug|GetStaticMeshComponent))
  (bind _relativelocation (Variables|/Script/Engine.SceneComponent|GetRelativeLocation _staticmeshcomponent))
  (bind _x (Math|Vector|BreakVector _relativelocation))
  (bind _returnvalue (Math|Float|Absolute(Float) _x))
  (if (Math|Boolean|ANDBoolean (>= _returnvalue 4.1e+02) (Variables|Default|GetCanHitEdge) (Math|Boolean|Equal(Boolean) (Variables|/Game/Blueprints/GameMode_SHUMP_Files/NewGameInstance.NewGameInstance_C|GetStopEverything (Variables|Default|GetInstance)) false))
    (Math|Float|NegateFloat _movementspeed
      (:%20%20
        (Variables|Default|SetCanHitEdge false))))
  (Transformation|SetRelativeLocation _staticmeshcomponent (+ _relativelocation (* (* (Math|Vector|MakeVector 1.0 0.0 0.0) _movementspeed) Delta%20Time)) false false)
  (if (<= _returnvalue 1e+01)
    (Variables|Default|SetCanHitEdge true)))