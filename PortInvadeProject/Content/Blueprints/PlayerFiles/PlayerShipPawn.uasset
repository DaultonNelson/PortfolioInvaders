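; Player ship pawn for an Invaders-style shooter, handling clamped horizontal movement, rate-limited laser fire and death.
; Game Instance holds lives, level and the StopEverything flag that gates input, while the controller's gameplay widget displays status.
; Being shot costs a life, triggers a tinted explosion, then resets or ends the game.
; Enemy collision, enabled after a startup delay, forces game over, which saves new high scores and schedules ChangeLevel.
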(event OnComponentBeginOverlap(PlayerShip)
  (params (OverlappedComponent :type Primitive%20Component%20Object%20Reference) (OtherActor :type Actor%20Object%20Reference) (OtherComp :type Primitive%20Component%20Object%20Reference) (OtherBodyIndex :type Integer) (bFromSweep :type Boolean) (SweepResult :type Hit%20Result%20Structure%20%28by%20ref%29))
  ;[1 1 1] On Collide With Enemy
  (if (Variables|Default|GetCanBeKilledByEnemy)
    (bind _asenemy_prefab (Utilities|Casting|CastToEnemyPrefab OtherActor))
    (Default|DeathBehavior _asenemy_prefab)
    (CallFunction|DeathBehavior)
    (Utilities|FlowControl|Delay 3.0)
    (CallFunction|GameOverBehavior)))

(event Collision|EventActorBeginOverlap
  (params (OtherActor :type Actor%20Object%20Reference)))

(event EventTick
  (params (DeltaSeconds :type Float%20%28single-precision%29)))

(event EventOnObjectShot
  ;[1 1 1] Killing the Player Ship
  (CallFunction|DeathBehavior)
  (Utilities|FlowControl|Delay 3.0)
  (if (> (Variables|/Game/Blueprints/GameMode_SHUMP_Files/NewGameInstance.NewGameInstance_C|GetPlayerLives (Variables|Default|GetInstance)) 0)
    (CallFunction|ResetShip)
    (else
      (CallFunction|GameOverBehavior))))

(event EventBeginPlay
  (bind _instance (Variables|Default|GetInstance))
  ;[1 1 1] Start
  (Math|Integer|IncrementInt (Variables|/Game/Blueprints/GameMode_SHUMP_Files/NewGameInstance.NewGameInstance_C|GetCurrentLevel _instance)
    (:%20%20
      (bind _ascustom_player_controller (Utilities|Casting|CastToCustomPlayerController (Game|GetPlayerController 0))
        (:then
          (Variables|Default|SetUIWidget (Variables|/Game/Blueprints/GameMode_SHUMP_Files/CustomPlayerController.CustomPlayerController_C|GetGameplayWidget _ascustom_player_controller))
          (Utilities|FlowControl|Delay 3.0)
          (Variables|/Game/Blueprints/GameMode_SHUMP_Files/NewGameInstance.NewGameInstance_C|SetStopEverything _instance false)
          (Rendering|Components|TextRender|SetText (Variables|/Game/UI/GameplayUI.GameplayUI_C|GetTextBlock_Ready (Variables|Default|GetUIWidget)) "")
          (Utilities|FlowControl|Delay 1e+01)
          (Variables|Default|SetCanBeKilledByEnemy true))
        (:CastFailed
          (Development|PrintString "Controller not found" true true "(R=0.537965,G=1.000000,B=0.538221,A=1.000000)" 99.0))))))

(event Input|ActionEvents|InputActionFire
  (params (Key :type Key%20Structure))
  ;[1 1 1] Shooting Lasers
  (:Released
    (if (and (Math|Boolean|Equal(Boolean) (Variables|/Game/Blueprints/GameMode_SHUMP_Files/NewGameInstance.NewGameInstance_C|GetStopEverything (Variables|Default|GetInstance)) false) (Variables|Default|GetCanFire))
      (Game|SpawnActorfromClass "/Game/Blueprints/PlayerFiles/Child_Laser_Blueprint_Player.Child_Laser_Blueprint_Player_C" (Transformation|GetWorldTransform (Variables|Default|GetMuzzle)) "Undefined" 0 0)
      (Variables|Default|SetCanFire false)
      (Utilities|FlowControl|Delay (Variables|Default|GetFireRate))
      (Variables|Default|SetCanFire true))))

(event Input|AxisEvents|InputAxisHorizontalAxis
  (params (AxisValue :type Float%20%28single-precision%29))
  (bind _playership (Variables|Default|GetPlayerShip))
  (bind _movementspeed (Variables|Default|GetMovementSpeed))
  (bind _clampvalue (Variables|Default|GetClampValue))
  (bind _returnvalue (Math|Vector|GetForwardVector _playership))
  (bind _returnvalue_2 (Math|Float|Absolute(Float) _clampvalue))
  (bind _relativelocation (Variables|/Script/Engine.SceneComponent|GetRelativeLocation _playership))
  (bind _returnvalue_3 (* _returnvalue AxisValue))
  (bind _returnvalue_4 (* _returnvalue_3 _movementspeed))
  (bind _returnvalue_5 (+ _returnvalue_4 _relativelocation))
  (bind (_x _y _z) (Math|Vector|BreakVector _returnvalue_5))
  ;[1 1 1] Ship Movement
  (if (Math|Boolean|Equal(Boolean) (Variables|/Game/Blueprints/GameMode_SHUMP_Files/NewGameInstance.NewGameInstance_C|GetStopEverything (Variables|Default|GetInstance)) false)
    (bind _result (Math|Float|NegateFloat _returnvalue_2)
      (:%20%20
        (Transformation|SetRelativeLocation _playership (Math|Vector|MakeVector (Math|Float|Clamp(Float) _x _result _returnvalue_2) _y _z) false false)))))

(fn ConstructionScript
  (bind _asnew_game_instance (Utilities|Casting|CastToNewGameInstance (Game|GetGameInstance)))
  (Variables|Default|SetInstance _asnew_game_instance))

(fn ResetShip
  (bind _playership (Variables|Default|GetPlayerShip))
  (bind _relativelocation (Variables|/Script/Engine.SceneComponent|GetRelativeLocation _playership))
  (bind (_x _y _z) (Math|Vector|BreakVector _relativelocation))
  (Transformation|SetRelativeLocation _playership (Math|Vector|MakeVector 0.0 _y _z) false false)
  (Rendering|ToggleVisibility (Variables|Default|GetPlayerShip) false)
  (Variables|Default|SetCanFire true))

(fn DeathBehavior
  (bind _explosion (Variables|Default|GetExplosion))
  (bind _instance (Variables|Default|GetInstance))
  (if (Math|Boolean|Equal(Boolean) (Variables|/Game/Blueprints/GameMode_SHUMP_Files/NewGameInstance.NewGameInstance_C|GetStopEverything _instance) false)
    (Variables|Default|SetCanFire false)
    (Math|Integer|DecrementInt (Variables|/Game/Blueprints/GameMode_SHUMP_Files/NewGameInstance.NewGameInstance_C|GetPlayerLives _instance)
      (:%20%20
        (Default|RebuildLives (Variables|Default|GetUIWidget))
        (Rendering|ToggleVisibility (Variables|Default|GetPlayerShip) false)
        (bind _returnvalue (Rendering|Material|CreateDynamicMaterialInstance _explosion 0 "/Game/Materials/FireworksDot_M.FireworksDot_M" "None" :!class /Script/Engine.PrimitiveComponent))
        (Rendering|Material|SetVectorParameterValue _returnvalue "Color" (Utilities|Struct|MakeLinearColor 0.0 1.0 0.0 1.0) :!class /Script/Engine.MaterialInstanceDynamic)
        (Rendering|Material|SetMaterial _explosion 0 _returnvalue)
        (Rendering|Material|SetMaterial _explosion 1 _returnvalue)
        (Components|Activation|Activate _explosion true)))))

(fn GameOverBehavior
  (bind _uiwidget (Variables|Default|GetUIWidget))
  (bind _instance (Variables|Default|GetInstance))
  (bind _savegamedata (Variables|/Game/Blueprints/GameMode_SHUMP_Files/NewGameInstance.NewGameInstance_C|GetSaveGameData _instance))
  (Variables|/Game/Blueprints/GameMode_SHUMP_Files/NewGameInstance.NewGameInstance_C|SetStopEverything _instance true)
  (Rendering|Components|TextRender|SetText (Variables|/Game/UI/GameplayUI.GameplayUI_C|GetTextBlock_GameOverLabel _uiwidget) "GAME OVER")
  (if (Variables|/Game/Blueprints/GameMode_SHUMP_Files/NewGameInstance.NewGameInstance_C|GetNewHighScore _instance)
    (Rendering|Components|TextRender|SetText (Variables|/Game/UI/GameplayUI.GameplayUI_C|GetTextBlock_NewHighScore _uiwidget) "NEW HI-SCORE GOT")
    (Variables|/Game/Blueprints/GameMode_SHUMP_Files/ShumpSaveGame.ShumpSaveGame_C|SetSavedHighScore _savegamedata (Variables|/Game/Blueprints/GameMode_SHUMP_Files/NewGameInstance.NewGameInstance_C|GetHighScore _instance))
    (SaveGame|SaveGametoSlot _savegamedata (Variables|/Game/Blueprints/GameMode_SHUMP_Files/NewGameInstance.NewGameInstance_C|GetSaveSlotName _instance)))
  (Utilities|Time|SetTimerbyFunctionName _instance "ChangeLevel" 3.0))