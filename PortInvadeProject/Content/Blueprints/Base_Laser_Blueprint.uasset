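; Base laser projectile Blueprint that provides movement and hit-filtering functions, with no event graph of its own to call them.
; LaserMovement moves the actor along its up vector by LaserSpeed scaled by delta time, without sweeping.
; OnLaserCollision checks the other actor for BPI_Shootable, stores a match in OverlappedActor or prints a red debug message otherwise, and returns the check result.
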(fn ConstructionScript)

(fn LaserMovement
  (params (DeltaTime :type Float%20%28single-precision%29))
  (Transformation|SetActorLocation (+ (* (* (Transformation|GetActorUpVector) (Variables|Default|GetLaserSpeed)) DeltaTime) (Transformation|GetActorLocation)) false false))

(fn OnLaserCollision
  (params (other :type Actor%20Object%20Reference))
  (bind _returnvalue (Utilities|DoesObjectImplementInterface other "/Game/Blueprints/BPI_Shootable.BPI_Shootable_C"))
  (if _returnvalue
    (Variables|Default|SetOverlappedActor other)
    (return _returnvalue)
    (else
      (Development|PrintString "Collided Object does not have shootable interface" true true "(R=1.000000,G=0.000000,B=0.000000,A=1.000000)" 5.0)
      (return _returnvalue))))