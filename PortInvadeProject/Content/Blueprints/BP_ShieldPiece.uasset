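; BP_ShieldPiece is a destructible shield segment that absorbs laser shots.
; On BeginPlay it creates a dynamic instance of the Shield material on its static mesh.
; Each overlap with a Base_Laser_Blueprint lowers PieceHealth and destroys the laser, tinting the mesh to DamagedColor while health remains and destroying the piece once it runs out.
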(event OnComponentBeginOverlap(StaticMeshComponent)
  (params (OverlappedComponent :type Primitive%20Component%20Object%20Reference) (OtherActor :type Actor%20Object%20Reference) (OtherComp :type Primitive%20Component%20Object%20Reference) (OtherBodyIndex :type Integer) (bFromSweep :type Boolean) (SweepResult :type Hit%20Result%20Structure%20%28by%20ref%29))
  (Utilities|Casting|CastToBase_Laser_Blueprint OtherActor
    (:then
      (Development|PrintString "HIT")
      (bind _result (Math|Integer|DecrementInt (Variables|Default|GetPieceHealth))
        (:%20%20
          (if (<= _result 0)
            (Actor|DestroyActor OtherActor)
            (Actor|DestroyActor)
            (else
              (Rendering|Material|SetVectorParameterValue (Variables|Default|GetMeshMaterial) "TextureColor" (Variables|Default|GetDamagedColor) :!class /Script/Engine.MaterialInstanceDynamic)
              (Actor|DestroyActor OtherActor))))))
    (:CastFailed
      (Development|PrintString "Not a laser"))))

(event EventBeginPlay
  (bind _returnvalue (Rendering|Material|CreateDynamicMaterialInstance (Variables|Debug|GetStaticMeshComponent) 0 "/Game/3DAssets/Shield/Shield.Shield" "None" :!class /Script/Engine.PrimitiveComponent))
  (Variables|Default|SetMeshMaterial _returnvalue))

(event EventOnObjectShot)

(fn ConstructionScript)